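; Player-controlled survivor that creates the HUD on BeginPlay, sets game-only input and handles weapon switching and reloading.
; Q refreshes owned and equipped flags through getters, then selects unarmed or pistol, or alternates pistol and shotgun with a ready sound when both are owned.
; Switching updates equipped flags and toggles weapon mesh visibility.
; R calls Reload, defined outside these graphs; both keys are ignored while reloading.
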(event `self.ReceiveBeginPlay`
  (bind _returnvalue (`|CreateWidget` "/Game/UI/WBP_HUD.WBP_HUD_C"))
  (`UserWidget.AddToViewport` _returnvalue 0)
  (`WidgetBlueprintLibrary.SetInputMode_GameOnly` (`GameplayStatics.GetPlayerController` 0)))

(event `Key|Q`
  (params (Key :type "Key Structure"))
  (:`Pressed`
    (if (not (`self.bIsReloading`))
      ; Initialize gun inventory variables
      (bind _returnvalue (`self.GetOwnsUnarmed`))
      (set `self.OwnsUnarmed` _returnvalue)
      (bind _returnvalue_2 (`self.GetOwnsPistol`))
      (set `self.OwnsPistol` _returnvalue_2)
      (bind _returnvalue_3 (`self.GetOwnsShotgun`))
      (set `self.OwnsShotgun` _returnvalue_3)
      (bind _returnvalue_4 (`self.GetUnarmedEquipped`))
      (set `self.UnarmedEquipped` _returnvalue_4)
      (bind _returnvalue_5 (`self.GetPistolEquipped`))
      (set `self.PistolEquipped` _returnvalue_5)
      (bind _returnvalue_6 (`self.GetShotgunEquipped`))
      (set `self.ShotgunEquipped` _returnvalue_6)
      ; If player does not own pistol or shotgun, just equip unarmed
      (if (and (`self.OwnsUnarmed`) (and (not (`self.OwnsPistol`)) (not (`self.OwnsShotgun`))))
        (`self.SetUnarmedEquipped` true)
        (`self.SetPistolEquipped` false)
        (`self.SetShotgunEquipped` false)
        (`SceneComponent.SetVisibility` (`self.ShotgunMeshModel`) false false)
        (`SceneComponent.SetVisibility` (`self.PistolMeshModel`) false false)
        (else
          ; Owns Pistol and Unarmed but not shotgun, always set Pistol to be equipped
          (if (and (and (`self.OwnsUnarmed`) (`self.OwnsPistol`)) (not (`self.OwnsShotgun`)))
            (`self.SetUnarmedEquipped` false)
            (`self.SetPistolEquipped` true)
            (`self.SetShotgunEquipped` false)
            (`SceneComponent.SetVisibility` (`self.ShotgunMeshModel`) false false)
            (`SceneComponent.SetVisibility` (`self.PistolMeshModel`) true false)
            (else
              ; Owns Pistol and Shotgun
              (if (and (and (`self.OwnsUnarmed`) (`self.OwnsPistol`)) (`self.OwnsShotgun`))
                (if (or (`self.UnarmedEquipped`) (`self.ShotgunEquipped`))
                  ;; Equip Pistol and show model
                  (`GameplayStatics.PlaySound2D` "/Game/Audio/GunSounds/PistolReady.PistolReady" 1.0 1.0 0.0 null null)
                  (`self.SetUnarmedEquipped` false)
                  (`self.SetPistolEquipped` true)
                  (`self.SetShotgunEquipped` false)
                  (`SceneComponent.SetVisibility` (`self.ShotgunMeshModel`) false false)
                  (`SceneComponent.SetVisibility` (`self.PistolMeshModel`) true false)
                  (else
                    ;; Equip Shotgun and show model
                    (`GameplayStatics.PlaySound2D` "/Game/Audio/GunSounds/ShotgunReady.ShotgunReady" 1.0 1.0 0.0 null null)
                    (`self.SetUnarmedEquipped` false)
                    (`self.SetPistolEquipped` false)
                    (`self.SetShotgunEquipped` true)
                    (`SceneComponent.SetVisibility` (`self.ShotgunMeshModel`) true false)
                    (`SceneComponent.SetVisibility` (`self.PistolMeshModel`) false false)))))))))))

(event `Key|R`
  (params (Key :type "Key Structure"))
  (:`Pressed`
    (if (not (`self.bIsReloading`))
      (`self.Reload`))))

(fn `UserConstructionScript`)