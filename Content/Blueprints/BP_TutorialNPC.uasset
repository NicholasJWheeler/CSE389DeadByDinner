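; Tutorial NPC that, on first interaction, arms the player's survivor with a loaded, equipped pistol and reserve ammo.
; BeginPlay caches the first BP_ControllableSurvivor found; Interact sets its weapon flags, swaps visible gun meshes and plays a ready sound.
; An interacted flag picks which prompt widget the proximity sphere shows while briefly pulsing a waving flag, noted as not yet properly connected.
; A separate spawn-area sphere toggles both widgets regardless of that flag.
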(event `self.ReceiveBeginPlay`
  (bind _outactors (`GameplayStatics.GetAllActorsOfClass` "/Game/Blueprints/BP_ControllableSurvivor.BP_ControllableSurvivor_C"))
  (for _array_element _outactors
    (set `self.SurvivorReference` _array_element)
    (break)))

(event `self.Sphere.OnComponentBeginOverlap`
  (params (OverlappedComponent :type "PrimitiveComponent Object Reference") (OtherActor :type "Actor Object Reference") (OtherComp :type "PrimitiveComponent Object Reference") (OtherBodyIndex :type Integer) (bFromSweep :type Boolean) (SweepResult :type "HitResult Structure (by ref)"))
  (if (not (`self.InteractedWithNPC`))
    (`SceneComponent.SetVisibility` (`self.Widget`) true false)
    ; Need to properly connect variable to make npc wave
    (set `self.WavingFlag` true)
    (`KismetSystemLibrary.Delay` 1.1)
    (set `self.WavingFlag` false)
    (else
      (`SceneComponent.SetVisibility` (`self.FinishedWidget`) true false)
      ; Need to properly connect variable to make npc wave
      (set `self.WavingFlag` true)
      (`KismetSystemLibrary.Delay` 1.1)
      (set `self.WavingFlag` false))))

(event `self.Sphere.OnComponentEndOverlap`
  (params (OverlappedComponent :type "PrimitiveComponent Object Reference") (OtherActor :type "Actor Object Reference") (OtherComp :type "PrimitiveComponent Object Reference") (OtherBodyIndex :type Integer))
  (if (not (`self.InteractedWithNPC`))
    (`SceneComponent.SetVisibility` (`self.Widget`) false false)
    (else
      (`SceneComponent.SetVisibility` (`self.FinishedWidget`) false false))))

(event `self.SpawnAreaSphere.OnComponentBeginOverlap`
  (params (OverlappedComponent :type "PrimitiveComponent Object Reference") (OtherActor :type "Actor Object Reference") (OtherComp :type "PrimitiveComponent Object Reference") (OtherBodyIndex :type Integer) (bFromSweep :type Boolean) (SweepResult :type "HitResult Structure (by ref)"))
  (`SceneComponent.SetVisibility` (`self.Widget`) true false)
  (`SceneComponent.SetVisibility` (`self.FinishedWidget`) true false))

(event `self.SpawnAreaSphere.OnComponentEndOverlap`
  (params (OverlappedComponent :type "PrimitiveComponent Object Reference") (OtherActor :type "Actor Object Reference") (OtherComp :type "PrimitiveComponent Object Reference") (OtherBodyIndex :type Integer))
  (`SceneComponent.SetVisibility` (`self.Widget`) false false)
  (`SceneComponent.SetVisibility` (`self.FinishedWidget`) false false))

(event `/Game/Blueprints/BPI_Interact.Interact`
  (bind _survivorreference (`self.SurvivorReference`))
  ; When first interacting with the tutorial NPC, equip the player with a pistol and bullets, and display the correct model. (Set next interaction boolean flag as well)
  (if (not (`self.InteractedWithNPC`))
    (set `self.InteractedWithNPC` true)
    (`ControllableSurvivor.SetOwnsPistol` _survivorreference true)
    (`ControllableSurvivor.SetPistolEquipped` _survivorreference true)
    (`ControllableSurvivor.SetUnarmedEquipped` _survivorreference false)
    (`ControllableSurvivor.SetShotgunEquipped` _survivorreference false)
    (`ControllableSurvivor.SetPistolLoadedAmmo` _survivorreference 9)
    (`ControllableSurvivor.SetPistolReserveAmmo` _survivorreference 108)
    (`GameplayStatics.PlaySound2D` "/Game/Audio/GunSounds/PistolReady.PistolReady" 1.0 1.0 0.0 null null)
    (`SceneComponent.SetVisibility` (`/Game/Blueprints/BP_ControllableSurvivor.ShotgunMeshModel` _survivorreference) false false)
    (`SceneComponent.SetVisibility` (`/Game/Blueprints/BP_ControllableSurvivor.PistolMeshModel` _survivorreference) true false)
    (`SceneComponent.SetVisibility` (`self.Widget`) false false)
    (`SceneComponent.SetVisibility` (`self.FinishedWidget`) true false)))

(fn `UserConstructionScript`)