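; Ammo merchant NPC that sells the survivor a pistol and shotgun ammo restock for skulls, which are tracked as the player's score.
; Sphere overlap toggles prompt or finished widgets and briefly pulses a waving flag, noted as not yet properly connected.
; Interact deducts the cost, sets loaded and reserve ammo, and plays a pickup sound, or shows an insufficient-skulls widget.
; The interacted flag only changes the overlap widget; repeat purchases remain possible.
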(event `self.ReceiveBeginPlay`
  (bind _outactors (`GameplayStatics.GetAllActorsOfClass` "/Game/Blueprints/BP_ControllableSurvivor.BP_ControllableSurvivor_C"))
  (for _array_element _outactors
    (set `self.SurvivorReference` _array_element)
    (break)))

(event `self.Sphere.OnComponentBeginOverlap`
  (params (OverlappedComponent :type "PrimitiveComponent Object Reference") (OtherActor :type "Actor Object Reference") (OtherComp :type "PrimitiveComponent Object Reference") (OtherBodyIndex :type Integer) (bFromSweep :type Boolean) (SweepResult :type "HitResult Structure (by ref)"))
  (`KismetSystemLibrary.IsObjectOfSoftClass` OtherActor "/Game/Blueprints/BP_ControllableSurvivor.BP_ControllableSurvivor_C"
    (:`True`
      (if (not (`self.InteractedWithNPC`))
        (`SceneComponent.SetVisibility` (`self.Widget`) true false)
        ; Need to properly connect variable to make npc wave
        (set `self.WavingFlag` true)
        (`KismetSystemLibrary.Delay` 1.1)
        (set `self.WavingFlag` false)
        (else
          (`SceneComponent.SetVisibility` (`self.FinishedWidget`) true false)
          ; Need to properly connect variable to make npc wave
          (set `self.WavingFlag` true)
          (`KismetSystemLibrary.Delay` 1.1)
          (set `self.WavingFlag` false))))))

(event `self.Sphere.OnComponentEndOverlap`
  (params (OverlappedComponent :type "PrimitiveComponent Object Reference") (OtherActor :type "Actor Object Reference") (OtherComp :type "PrimitiveComponent Object Reference") (OtherBodyIndex :type Integer))
  (bind _insufficientskullswidget (`self.InsufficientSkullsWidget`))
  (`KismetSystemLibrary.IsObjectOfSoftClass` OtherActor "/Game/Blueprints/BP_ControllableSurvivor.BP_ControllableSurvivor_C"
    (:`True`
      (if (not (`self.InteractedWithNPC`))
        (`SceneComponent.SetVisibility` (`self.Widget`) false false)
        (`SceneComponent.SetVisibility` _insufficientskullswidget false false)
        (else
          (`SceneComponent.SetVisibility` (`self.FinishedWidget`) false false)
          (`SceneComponent.SetVisibility` _insufficientskullswidget false false))))))

(event `self.Interact`
  (bind _survivorreference (`self.SurvivorReference`))
  ; When first interacting with the ammo NPC, if they have enough skulls to give up, equip the player with full ammo reserves and full loaded guns, and display the correct model. (Set next interaction boolean flag as well)
  (bind _returnvalue (`ControllableSurvivor.GetScore` _survivorreference))
  (if (>= _returnvalue 3)
    (if true
      (set `self.InteractedWithNPC` true)
      ; Subtract 3 Skulls to pay merchant for ammo restock
      (bind _returnvalue_2 (`ControllableSurvivor.GetScore` _survivorreference))
      (`ControllableSurvivor.SetScore` _survivorreference (- _returnvalue_2 3))
      (`ControllableSurvivor.SetPistolLoadedAmmo` _survivorreference 9)
      (`ControllableSurvivor.SetPistolReserveAmmo` _survivorreference 180)
      (`ControllableSurvivor.SetShotgunLoadedAmmo` _survivorreference 5)
      (`ControllableSurvivor.SetShotgunReserveAmmo` _survivorreference 60)
      (`GameplayStatics.PlaySound2D` "/Game/Audio/FX/itemPickup.itemPickup" 1.0 1.0 0.0 null null)
      (`SceneComponent.SetVisibility` (`self.Widget`) false false)
      (`SceneComponent.SetVisibility` (`self.FinishedWidget`) true false)
      (`SceneComponent.SetVisibility` (`self.InsufficientSkullsWidget`) false false))
    (else
      ; Tell player they do not have enough skulls
      (`SceneComponent.SetVisibility` (`self.Widget`) false false)
      (`SceneComponent.SetVisibility` (`self.FinishedWidget`) false false)
      (`SceneComponent.SetVisibility` (`self.InsufficientSkullsWidget`) true false))))

(fn `UserConstructionScript`)